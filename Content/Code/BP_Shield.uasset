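; BP_Shield is a randomly meshed pickup that the player drags with telekinesis and drops as a projectile-absorbing shield.
; It can drift toward PlayerLocation until clicked, then a gated Tick interpolates it toward the cursor while a looping timer drains BP_Brain's Telekinesis.
; Release swaps to the shield mesh and deploys it.
; Touching the brain, or any non-shield while undeployed, destroys it; once deployed, projectiles deplete its Health.
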(event `self.ReceiveTick`
  (params (DeltaSeconds :type "Float (single-precision)"))
  (if (`self.moveTowardsPlayer`)
    (`self.K2_SetActorLocation` (`KismetMathLibrary.VInterpTo` (`self.K2_GetActorLocation`) (`self.PlayerLocation`) DeltaSeconds 1.0))
    (else
      (`/Engine/EditorBlueprintResources/StandardMacros.Gate` true :!label _label
        (:`Exit`
          (`self.K2_SetActorLocation` (`KismetMathLibrary.VInterpTo` (`KismetMathLibrary.MakeVector` (.x (`self.K2_GetActorLocation`)) (.y (`self.K2_GetActorLocation`))) (`KismetMathLibrary.MakeVector` (.x (`.Location` (`GameplayStatics.BreakHitResult` (`PlayerController.GetHitResultUnderCursorByChannel` (`GameplayStatics.GetPlayerController` 0) "TraceTypeQuery1" true)))) (.y (`.Location` (`GameplayStatics.BreakHitResult` (`PlayerController.GetHitResultUnderCursorByChannel` (`GameplayStatics.GetPlayerController` 0) "TraceTypeQuery1" true))))) (`GameplayStatics.GetWorldDeltaSeconds`) 3.0)))))))

(event `self.ReceiveDestroyed`
  (if (not (== (stale `self.StaticMesh.OnClicked` _returnvalue) null))
    (`AudioComponent.Stop` (stale `self.StaticMesh.OnClicked` _returnvalue))))

(event `self.StaticMesh.OnClicked`
  (params (TouchedComponent :type "PrimitiveComponent Object Reference") (ButtonPressed :type "Key Structure"))
  (if (not (`self.isShieldDeployed`))
    (bind _returnvalue (`GameplayStatics.CreateSound2D` "/Game/Sound/Telekinesis.Telekinesis" 1.0 1.0 0.0 null))
    (`AudioComponent.Play` _returnvalue 0.0)
    (set `PlayerController.bEnableMouseOverEvents` false (`GameplayStatics.GetPlayerController` 0))
    (set `self.moveTowardsPlayer` false)
    (set `self.isShieldDeployed` false)
    (bind _returnvalue_2 (`KismetSystemLibrary.K2_SetTimerDelegate` (delegate `ConsumeTelekinesis`) 0.5 true))
    (goto _label :!via `Open`)))

(event `self.StaticMesh.OnReleased`
  (params (TouchedComponent :type "PrimitiveComponent Object Reference") (ButtonReleased :type "Key Structure"))
  (`StaticMeshComponent.SetStaticMesh` (`self.StaticMesh`) "/Game/Lewis/ShieldPickup.ShieldPickup")
  (`self.SetActorScale3D` (20.0 20.0 20.0))
  (if (`AudioComponent.IsPlaying` (stale `self.StaticMesh.OnClicked` _returnvalue))
    (`AudioComponent.Stop` (stale `self.StaticMesh.OnClicked` _returnvalue))
    (`GameplayStatics.PlaySound2D` "/Game/Sound/ShieldDeploy.ShieldDeploy" 1.0 1.0 0.0 null null)
    (set `PlayerController.bEnableMouseOverEvents` true (`GameplayStatics.GetPlayerController` 0))
    (set `self.isShieldDeployed` true)
    (`KismetSystemLibrary.K2_PauseTimerHandle` (stale `self.StaticMesh.OnClicked` _returnvalue_2))
    (goto _label :!via `Close`)))

(event `ConsumeTelekinesis`
  (bind _asbp_brain (cast `/Game/Code/BP_Brain` (`Controller.K2_GetPawn` (`GameplayStatics.GetPlayerController` 0))))
  (set `/Game/Code/BP_Brain.Telekinesis` (- (`/Game/Code/BP_Brain.Telekinesis` _asbp_brain) 1.0) _asbp_brain))

(event `self.StaticMesh.OnComponentBeginOverlap`
  (params (OverlappedComponent :type "PrimitiveComponent Object Reference") (OtherActor :type "Actor Object Reference") (OtherComp :type "PrimitiveComponent Object Reference") (OtherBodyIndex :type Integer) (bFromSweep :type Boolean) (SweepResult :type "HitResult Structure (by ref)"))
  ;[1 1 1] take damage
  (cast `/Game/Code/BP_Shield` OtherActor
    (:`CastFailed`
      (cast `/Game/Code/BP_Brain` OtherActor
        (:`then`
          (`self.K2_DestroyActor` :!label _label_2))
        (:`CastFailed`
          (`GameplayStatics.PlaySound2D` "/Game/Sound/ShieldHit.ShieldHit" 1.0 1.0 0.0 null null)
          (if (`self.isShieldDeployed`)
            (cast `/Game/Code/BP_Projectile` OtherActor)
            (bind _output_get (set `self.Health` (- (`self.Health`) 5.0)))
            (if (<= _output_get 0.0)
              (`self.K2_DestroyActor`))
            (else
              (goto _label_2))))))))

(fn `UserConstructionScript`
  (bind _meshes (`self.Meshes`))
  (`StaticMeshComponent.SetStaticMesh` (`self.StaticMesh`) (`|GetArrayItem` _meshes (`KismetMathLibrary.RandomIntegerInRange` 0 (- (`KismetArrayLibrary.Array_Length` _meshes) 1)))))