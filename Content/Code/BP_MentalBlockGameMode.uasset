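; Game mode for Mental Block that spawns bad-thought projectiles and shields around the player and tracks survival time.
; Tick counts down a spawn timer, then makes a 50/50 pick between the two, passing in the player's location.
; Spawn points come from randomly indexed BP_ProjectileSpawner actors, jittered along X or Y according to a spawner's Y position.
; A looping one-second timer increments TimeScore and shortens the spawn gap every 30 seconds.
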(event `self.ReceiveBeginPlay`
  (set `self.SpawnTimer` (`self.ProjectileSpawnGap`))
  (bind _outactors (`GameplayStatics.GetAllActorsOfClass` "/Game/Code/BP_ProjectileSpawner.BP_ProjectileSpawner_C"))
  (set `self.Spawners` _outactors)
  (`KismetSystemLibrary.K2_SetTimerDelegate` (delegate `GameTimer`) 1.0 true))

(event `GameTimer`
  ;[1 1 1] score timer
  (set `self.timeScore` (+ (`self.timeScore`) 1.0))
  (if (== (mod (`self.timeScore`) 30.0) 0.0)
    (set `self.ProjectileSpawnGap` (- (`self.ProjectileSpawnGap`) 0.2))))

(event `self.ReceiveTick`
  (params (DeltaSeconds :type "Float (single-precision)"))
  (bind _spawners (`self.Spawners`))
  (bind _returnvalue (`self.K2_GetActorLocation` (`GameplayStatics.GetPlayerPawn` 0)))
  (bind _returnvalue_2 (`self.K2_GetActorLocation` (`GameplayStatics.GetPlayerPawn` 0)))
  (bind _output (`|GetArrayItem` _spawners (`KismetMathLibrary.RandomIntegerInRange` 0 (- (`KismetArrayLibrary.Array_Length` _spawners) 1))))
  (bind (_returnvalue_x _returnvalue_y) (`KismetMathLibrary.BreakVector` (`self.K2_GetActorLocation` _output)))
  (bind (_returnvalue_x_2 _returnvalue_y_2) (`KismetMathLibrary.BreakVector` (`self.K2_GetActorLocation` _output)))
  (bind (_returnvalue_x_3 _returnvalue_y_3) (`KismetMathLibrary.BreakVector` (`self.K2_GetActorLocation` _output)))
  (bind _returnvalue_3 (+ (`KismetMathLibrary.RandomFloatInRange` -2000.0 2000.0) _returnvalue_y))
  (bind _returnvalue_4 (+ (`KismetMathLibrary.RandomFloatInRange` -2000.0 2000.0) _returnvalue_x_2))
  (bind _output_get (set `self.SpawnTimer` (- (`self.SpawnTimer`) DeltaSeconds)))
  (if (< _output_get 0.0)
    (`/Engine/EditorBlueprintResources/StandardMacros.DoOnce` false :!label _label
      (:`Completed`
        (set `self.spawnBadThought` (>= (`KismetMathLibrary.RandomIntegerInRange` 0 100) 50))
        (if (>= (`KismetMathLibrary.Abs` _returnvalue_y_3) 2000.0)
          (if (`self.spawnBadThought`)
            (`|SpawnActorFromClass` "/Game/Code/BP_Projectile.BP_Projectile_C" (`KismetMathLibrary.MakeTransform` (`KismetMathLibrary.MakeVector` _returnvalue_4 _returnvalue_y_2) (struct) (10.0 10.0 10.0)) "Undefined" "OverrideRootScale" null _returnvalue_2 null)
            (else
              (`|SpawnActorFromClass` "/Game/Code/BP_Shield.BP_Shield_C" (`KismetMathLibrary.MakeTransform` (`KismetMathLibrary.MakeVector` _returnvalue_4 _returnvalue_y_2) (struct) (20.0 20.0 20.0)) "Undefined" "OverrideRootScale" null _returnvalue_2 null)))
          (elif (`self.spawnBadThought`)
            (`|SpawnActorFromClass` "/Game/Code/BP_Projectile.BP_Projectile_C" (`KismetMathLibrary.MakeTransform` (`KismetMathLibrary.MakeVector` _returnvalue_x _returnvalue_3) (struct) (10.0 10.0 10.0)) "Undefined" "OverrideRootScale" null _returnvalue null)
            (else
              (`|SpawnActorFromClass` "/Game/Code/BP_Shield.BP_Shield_C" (`KismetMathLibrary.MakeTransform` (`KismetMathLibrary.MakeVector` _returnvalue_x _returnvalue_3) (struct) (20.0 20.0 20.0)) "Undefined" "OverrideRootScale" null _returnvalue null))))
        (set `self.SpawnTimer` (`self.ProjectileSpawnGap`))))
    (else
      (goto _label :!via `Reset`))))

(fn `UserConstructionScript`)