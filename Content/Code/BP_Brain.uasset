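; BP_Brain is the actor that holds the Telekinesis meter, which acts as health, and puts the BP_InGameUI widget on screen at BeginPlay.
; Static mesh overlaps drive the meter: a BP_Shield raises it and is destroyed, while a BP_Projectile lowers it.
; An empty meter only prints GAME OVER.
; Physics-handle grabbing and cursor-aimed, rate-limited shield spawning remain as unconnected nodes that never run.
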(event `self.ReceiveBeginPlay`
  (bind _returnvalue (`|CreateWidget` "/Game/UI/BP_InGameUI.BP_InGameUI_C" (`GameplayStatics.GetPlayerController` 0)))
  (`UserWidget.AddToViewport` _returnvalue 0))

(event `Key|LeftMouseButton`
  (params (Key :type "Key Structure")))

(event `self.StaticMesh.OnComponentBeginOverlap`
  (params (OverlappedComponent :type "PrimitiveComponent Object Reference") (OtherActor :type "Actor Object Reference") (OtherComp :type "PrimitiveComponent Object Reference") (OtherBodyIndex :type Integer) (bFromSweep :type Boolean) (SweepResult :type "HitResult Structure (by ref)"))
  (bind _asbp_shield (cast `/Game/Code/BP_Shield` OtherActor)
    (:`then`
      (set `self.Telekinesis` (+ (`self.Telekinesis`) 5.0))
      (`self.K2_DestroyActor` _asbp_shield))
    (:`CastFailed`
      ;[1 1 1] take damage
      (cast `/Game/Code/BP_Projectile` OtherActor)
      (set `self.Telekinesis` (- (`self.Telekinesis`) 5.0))
      ;[1 1 1] Game over
      (if (<= (`self.Telekinesis`) 0.0)
        (`KismetSystemLibrary.PrintString` "GAME OVER" true true (struct :`R` 1.0 :`B` 0.00682 :`A` 1.0))))))

(fn `UserConstructionScript`)